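; MyBasicCharacter is a character Blueprint that exercises attribute functions and prints the results for debugging.
; On BeginPlay it prints Health, Strength, Intelligence, Agility, the sum of the latter three, and Damage.
; It then calls ImproveStrength twice, first with zero and then with a variable, printing Strength after each call.
; The getters and ImproveStrength are not defined in these graphs, and the Construction Script is empty.
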(event `self.ReceiveBeginPlay`
  (bind _returnvalue (`self.GetHealth`))
  (`KismetSystemLibrary.PrintString` (`KismetStringLibrary.Conv_IntToString` _returnvalue))
  (bind _returnvalue_2 (`self.GetStrength`))
  (`KismetSystemLibrary.PrintString` (`KismetStringLibrary.Concat_StrStr` "Strength:" (`KismetStringLibrary.Conv_IntToString` _returnvalue_2)))
  (bind _returnvalue_3 (`self.GetIntelligence`))
  (`KismetSystemLibrary.PrintString` (`KismetStringLibrary.Concat_StrStr` "Intelligence" (`KismetStringLibrary.Conv_IntToString` _returnvalue_3)))
  (bind _returnvalue_4 (`self.GetAgility`))
  (`KismetSystemLibrary.PrintString` (`KismetStringLibrary.Concat_StrStr` "Agility" (`KismetStringLibrary.Conv_IntToString` _returnvalue_4)))
  (`KismetSystemLibrary.PrintString` (`KismetStringLibrary.Conv_IntToString` (+ _returnvalue_2 _returnvalue_3 _returnvalue_4)))
  (bind _returnvalue_5 (`self.GetDamage`))
  (`KismetSystemLibrary.PrintString` (`KismetStringLibrary.Concat_StrStr` "Damage:" (`KismetStringLibrary.Conv_IntToString` _returnvalue_5)))
  (`self.ImproveStrength` 0)
  (bind _returnvalue_6 (`self.GetStrength`))
  (`KismetSystemLibrary.PrintString` (`KismetStringLibrary.Conv_IntToString` _returnvalue_6))
  (`self.ImproveStrength` (`self.NewVar_2`))
  (bind _returnvalue_7 (`self.GetStrength`))
  (`KismetSystemLibrary.PrintString` (`KismetStringLibrary.Conv_IntToString` _returnvalue_7)))

(event `self.ReceiveActorBeginOverlap`
  (params (OtherActor :type "Actor Object Reference")))

(event `self.ReceiveTick`
  (params (DeltaSeconds :type "Float (single-precision)")))

(fn `UserConstructionScript`)